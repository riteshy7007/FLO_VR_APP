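; BP_Anchor is a UXT mixed reality anchor actor that the user places and pins in the world, named with a random color-number label if none is set.
; AddInteractionComponent adds either manual grab or tap-to-place.
; Ending placement saves the anchor through BP_Pawn and destroys BoundControl.
; A remove button asks BP_Pawn to delete the anchor, and Tick smoothly turns the buttons toward the camera.
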(event Custom|OnButtonPressed
  (params (Button :type Uxt%20Pressable%20Button%20Component%20Object%20Reference) (Pointer :type Uxt%20Pointer%20Component%20Object%20Reference))
  ;[1 1 1] When the user pressed a button, check which button and call appropriate event
  (CallFunction|RemoveAnchor))

(event Custom|RemoveAnchor
  ;[1 1 1] Communicate to Pawn and destroy
  (bind _asbp_pawn (Utilities|Casting|CastToBP_Pawn (Game|Player|GetPlayerPawn 0)))
  (Default|DeleteLocalAnchor _asbp_pawn (Utilities|String|StringToName (Variables|Default|GetAnchorName)) self))

(event Custom|Bind%20Button%20Press
  ;[1 1 1] When the user pressed a button, check which button and call appropriate event
  (bind _asuxt_pressable_button_actor (Utilities|Casting|CastToUxtPressableButtonActor (Variables|/Script/Engine.ChildActorComponent|GetChildActor (Variables|Default|GetChildActor_RemoveAnchor))))
  (EventDispatchers|AssignOnButtonPressed (Variables|/Script/UXTools.UxtBasePressableButtonActor|GetButtonComponent _asuxt_pressable_button_actor) (delegate Custom|OnButtonPressed)))

(event Custom|AddInteractionComponent
  (params (PlacementType :type Integer))
  ;[1 1 1] Add a way for the user to move the anchor to the correct location
  (switch int PlacementType
    (:0
      ;[1 1 1] If user chose 'Manual' they will need to move the anchor from near or far and when they let go, it will save
      (bind _returnvalue (AddComponent|AddUxtGenericManipulatorComponent false))
      (EventDispatchers|BindEventtoOnEndGrab _returnvalue (delegate Custom|User%20Ends%20Grab)))
    (:1
      ;[1 1 1] If the user chooses Tap and Place, the must tap on the Blueprint and it will lock to head gaze's front direction. When line trace intersects with a collision, the Blueprint will snap to that hit point. When they are ready, they can press their fingers to confirm the location
      (bind _returnvalue_2 (AddComponent|AddUxtTaptoPlaceComponent))
      (EventDispatchers|BindEventtoOnEndPlacing _returnvalue_2 (delegate Custom|User%20Ends%20Placing)))))

(event Custom|SaveAnchorTransform
  ;[1 1 1] Will save the anchor's transform
  (bind _asbp_pawn (Utilities|Casting|CastToBP_Pawn (Game|Player|GetPlayerPawn 0)))
  (Default|SaveLocalAnchor _asbp_pawn (Variables|Default|GetAnchor) (Utilities|String|StringToName (Variables|Default|GetAnchorName)))
  ;[1 1 1] ToPrevent any further manipulation by the user
  (Components|DestroyComponent (Variables|Default|GetBoundControl)))

(event Custom|User%20Ends%20Placing
  (params (TapToPlace :type Uxt%20Tap%20to%20Place%20Component%20Object%20Reference))
  ;[1 1 1] If the user chooses Tap and Place, the must tap on the Blueprint and it will lock to head gaze's front direction. When line trace intersects with a collision, the Blueprint will snap to that hit point. When they are ready, they can press their fingers to confirm the location
  (CallFunction|SaveAnchorTransform))

(event Custom|User%20Ends%20Grab
  (params (Grabbable :type Uxt%20Grab%20Target%20Component%20Object%20Reference) (GrabPointer :type Uxt%20Grab%20Pointer%20Data%20Structure))
  ;[1 1 1] If user chose 'Manual' they will need to move the anchor from near or far and when they let go, it will save
  (CallFunction|SaveAnchorTransform))

(event EventBeginPlay
  ;[1 1 1] When spawned, will check if it was given a name and if not, will generate a new name. If it was changed, but should still generate a
  (if (or (Utilities|Enum|Equal(Enum) (Variables|Default|GetAnchorName) "None") (Utilities|Array|IsEmpty (Variables|Default|GetAnchorName)))
    (bind _new_name (CallFunction|GenerateRandomName))
    (Variables|Default|SetAnchorName _new_name))
  (Rendering|Components|TextRender|SetText (Variables|Default|GetUxtTextRender) (Utilities|Text|ToText(String) (Variables|Default|GetAnchorName)))
  ;[1 1 1] Prepare Anchor's button
  (CallFunction|BindButtonPress))

(event EventTick
  (params (DeltaSeconds :type Float%20%28single-precision%29))
  (bind _scene_anchorbuttons (Variables|Default|GetScene_AnchorButtons))
  ;[1 1 1] Smoothly rotate to face the user. Just in case the anchor gets placed in a location that the user cannot reach or see properly
  (Transformation|SetWorldRotation _scene_anchorbuttons (Math|Interpolation|RInterpTo (Transformation|GetWorldRotation _scene_anchorbuttons) (Math|Rotator|FindLookatRotation (Transformation|GetWorldLocation _scene_anchorbuttons) (Transformation|GetWorldLocation (Variables|/Game/WorldBuilder/Blueprint/Pawns/BP_Pawn.BP_Pawn_C|GetCamera (.AsBP%20Pawn (Utilities|Casting|CastToBP_Pawn (Game|Player|GetPlayerPawn 0)))))) DeltaSeconds 2.0) false false))

(fn ConstructionScript)

(fn GenerateRandomName
  (bind _nameoptions___color (Variables|Default|GetNameOptions%20-%20Color))
  (bind _nameoptions___number (Variables|Default|GetNameOptions%20-%20Number))
  ;[1 1 1] Will append the two random indices with a " - " seperator
  (return (Utilities|String|Append (Utilities|Array|Get(acopy) _nameoptions___color (Math|Random|RandomIntegerinRange 0 (Utilities|Array|LastIndex _nameoptions___color))) "-" (Utilities|Array|Get(acopy) _nameoptions___number (Math|Random|RandomIntegerinRange 0 (Utilities|Array|LastIndex _nameoptions___number))))))