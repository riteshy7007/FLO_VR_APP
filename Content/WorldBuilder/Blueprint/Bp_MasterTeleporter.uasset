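; Master teleporter gate that moves AI characters between gates linked by ID.
; When active, a character overlapping its box broadcasts the SendingTo ID and that character to all BPi_HoloLens interface actors.
; Its TeleportCharacter event checks the ID, moves AI_Friend characters to its Out point and calls Search.
; Delayed collision toggles aim to switch the receiving box off briefly around arrival.
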(event OnComponentBeginOverlap(Box)
  (params (OverlappedComponent :type Primitive%20Component%20Object%20Reference) (OtherActor :type Actor%20Object%20Reference) (OtherComp :type Primitive%20Component%20Object%20Reference) (OtherBodyIndex :type Integer) (bFromSweep :type Boolean) (SweepResult :type Hit%20Result%20Structure%20%28by%20ref%29))
  ;[1 1 1] If the gate is active: When the AI overlaps with the box, teleport them to a gate with a specific ID
  (if (Variables|Teleport|GetGateActive)
    (bind _ascharacter (Utilities|Casting|CastToCharacter OtherActor))
    (bind _outactors (Actor|GetAllActorswithInterface "/Game/WorldBuilder/Blueprint/Core/BPi_HoloLens.BPi_HoloLens_C"))
    (for _array_element _outactors
      (Class|BPiHoloLens|TeleportCharacter(Message) _array_element (Variables|Teleport|GetSendingTo) _ascharacter))))

(event Custom|SetCollisionEnabledAfterDelay
  (params (Duration :type Float%20%28single-precision%29) (NewType :type ECollisionEnabled%20Enum :default "NoCollision"))
  ;[1 1 1] Toggle Collision
  (Utilities|FlowControl|Delay Duration)
  (Collision|SetCollisionEnabled (Variables|Default|GetBox) NewType))

(event EventTeleportCharacter
  (params (Teleporter%20ID :type Integer) (IncomingAI :type Character%20Object%20Reference))
  ;[1 1 1] An AI Overlapped another teleporter. Check if this ID is the one it is being sent to
  (if (== Teleporter%20ID (Variables|Teleport|GetTeleporterID))
    ;[1 1 1] Make sure the Blueprint inherits from AI_Friend
    (bind _asai_friend (Utilities|Casting|CastToAI_Friend IncomingAI))
    ;[1 1 1] Set collision off
    (CallFunction|SetCollisionEnabledAfterDelay 0.0 "NoCollision")
    ;[1 1 1] Teleport the character to the new location and call Search
    (Transformation|SetActorLocation _asai_friend (.location (Transformation|GetWorldTransform (Variables|Default|GetOut))) false false)
    (Default|Search _asai_friend)
    ;[1 1 1] Return Collision after 2 seconds
    (CallFunction|SetCollisionEnabledAfterDelay 2.0 "QueryOnly")))

(fn ConstructionScript)