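; BP_Ramp is a ramp actor whose Mover component deploys to the actor pivot when triggered by a motion sensor or by the pawn's voice interaction.
; Sensor calls step it slowly toward the pivot, while voice calls snap it there instantly.
; A retriggerable delay detects when sensor calls stop, then starts a looping timer that quickly retracts it to the DistanceToMove offset and pauses.
; The construction script sets the initial position from Open.
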(event Custom|MoveRamp
  (bind _returnvalue (Transformation|GetActorLocation))
  (bind _mover (Variables|Default|GetMover))
  (bind _returnvalue_2 (Transformation|GetWorldLocation _mover))
  ;[1 1 1] When called, will slowly move the Mover back to the parent actor's pivot
  (Utilities|FlowControl|Sequence
    (:then_0
      ;;[1 1 1] Only move if not equal
      (if (Math|Vector|NotEqual(Vector) _returnvalue_2 _returnvalue 0.5)
        (Transformation|SetWorldLocation _mover (Math|Interpolation|VInterptoConstant _returnvalue_2 _returnvalue (Utilities|Time|GetWorldDeltaSeconds) 1e+01) false false)))
    (:then_1
      ;[1 1 1] Has the ramp been fully deployed
      (Utilities|FlowControl|RetriggerableDelay 0.1)
      ;[1 1 1] If Ramp is not fully out, call CloseRamp ever .02 to retract it back
      (bind _returnvalue_3 (Utilities|Time|SetTimerbyEvent (EventDispatchers|CreateEvent :!event Custom|CloseRamp) 0.02 true))
      (Variables|Default|SetRamp_Timer _returnvalue_3))))

(event Custom|CloseRamp
  (bind _returnvalue (Transformation|GetActorLocation))
  (bind _distancetomove (Variables|Default|GetDistanceToMove))
  (bind _mover (Variables|Default|GetMover))
  (bind _returnvalue_2 (Transformation|GetWorldLocation _mover))
  (bind _returnvalue_3 (+ _returnvalue _distancetomove))
  ;[1 1 1] Return the ramp to the starting offset very quickly
  (if (Math|Vector|NotEqual(Vector) _returnvalue_2 _returnvalue_3 0.5)
    (Transformation|SetWorldLocation _mover (Math|Interpolation|VInterptoConstant _returnvalue_2 _returnvalue_3 (Utilities|Time|GetWorldDeltaSeconds) 1e+02) false false)
    (else
      (Utilities|Time|PauseTimerbyHandle (Variables|Default|GetRamp_Timer)))))

(event EventInteractwithObject
  (params (RightHand :type Boolean))
  ;[1 1 1] If False, called from BP_MotionSensor
  ; If True, called from BP_Pawn using Voice
  (if RightHand
    ;[1 1 1] Forcing the ramp to open without animation
    (Transformation|SetWorldLocation (Variables|Default|GetMover) (Transformation|GetActorLocation) false false)
    (else
      (CallFunction|MoveRamp))))

(fn ConstructionScript
  (Transformation|SetWorldLocation (Variables|Default|GetMover) (Math|Vector|SelectVector (+ (Transformation|GetWorldLocation (Variables|Default|GetMover)) (Variables|Default|GetDistanceToMove)) (Transformation|GetActorLocation) (Variables|Default|GetOpen)) false false))