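; World-builder spawnable kit piece that shows a floor, ramp, wall or roof mesh chosen by the ESpawnable enum.
; BP_ObjectSpawner calls CycleSpawnable to step the enum up or down with wraparound and refresh the mesh, which the construction script also sets.
; Each mesh is re-centered on the actor using its bounds, with its top at the origin.
; HasBeenSpawned adds a UXT generic manipulator to enable interaction.
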(event Custom|CycleSpawnable
  (params (Up :type Boolean))
  ;[1 1 1] Called by BP_ObjectSpawner
  (CallFunction|CycleMeshes Up)
  (CallFunction|SetandPlaceMesh))

(event Custom|HasBeenSpawned
  ;[1 1 1] WhenSpawned, enable interaction
  (AddComponent|AddUxtGenericManipulatorComponent))

(fn ConstructionScript
  (CallFunction|SetandPlaceMesh))

(fn SetandPlaceMesh
  (bind _staticmesh (Variables|Default|GetStaticMesh))
  (bind _staticmesh_2 (Variables|Default|GetStaticMesh))
  (bind (_origin _boxextent) (Collision|GetComponentBounds _staticmesh_2))
  ;[1 1 1] Set the static mesh based on the value of ESpawnable
  (Components|StaticMesh|SetStaticMesh _staticmesh (Utilities|Select :Index (Variables|Default|GetESpawnable) :NewEnumerator0 "/Game/WorldBuilder/Assets/Architecture/Kit_Floor/Mesh/SM_Kit_Floor.SM_Kit_Floor" :NewEnumerator1 "/Game/WorldBuilder/Assets/Architecture/Kit_Ramp/Mesh/SM_Kit_Ramp.SM_Kit_Ramp" :NewEnumerator2 "/Game/WorldBuilder/Assets/Architecture/Kit_Wall/Mesh/SM_Kit_Wall_Straight.SM_Kit_Wall_Straight" :NewEnumerator3 "/Game/WorldBuilder/Assets/Architecture/Kit_Roof/Mesh/SM_Kit_Roof_Corner_In.SM_Kit_Roof_Corner_In" :NewEnumerator4 "/Game/WorldBuilder/Assets/Architecture/Kit_Roof/Mesh/SM_Kit_Roof_Corner_Out.SM_Kit_Roof_Corner_Out" :NewEnumerator5 "/Game/WorldBuilder/Assets/Architecture/Kit_Roof/Mesh/SM_Kit_Roof_Straight.SM_Kit_Roof_Straight"))
  ;[1 1 1] Reset the location back to 0,0,0
  (Transformation|SetRelativeLocation _staticmesh "0, 0, 0" false false)
  ;[1 1 1] Place centered in the Blueprint while keeping the Z below 0 and the object facing the best direction
  (Transformation|AddWorldOffset _staticmesh_2 (- (- (Transformation|GetWorldLocation _staticmesh_2) _origin) (Math|Vector|MakeVector 0.0 0.0 (.z _boxextent))) false false))

(fn CycleMeshes
  (params (Up :type Boolean))
  (if Up
    (if (>= (Variables|Default|GetESpawnable) (Math|Conversions|ToByte(Integer) (- (|GetNumEnumEntries) 1)))
      ;[1 1 1] If max value, set to 0
      (Variables|Default|SetESpawnable (Utilities|Enum|ByteToEnumESpawnableType))
      (else
        ;[1 1 1] If not max, add one
        (Variables|Default|SetESpawnable (Utilities|Enum|ByteToEnumESpawnableType (+ (Variables|Default|GetESpawnable) 1)))))
    (elif (== (Variables|Default|GetESpawnable) 0)
      ;[1 1 1] If value is 0, set to max
      (Variables|Default|SetESpawnable (Utilities|Enum|ByteToEnumESpawnableType (Math|Conversions|ToByte(Integer) (- (|GetNumEnumEntries) 1))))
      (else
        ;[1 1 1] If not 0, subtract by 1
        (Variables|Default|SetESpawnable (Utilities|Enum|ByteToEnumESpawnableType (- (Variables|Default|GetESpawnable) 1)))))))