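; BP_TeleportGate is a world gate actor with an active/inactive state shown by color and reflected in navigation; the file contains no teleport logic.
; The ToggleGate event stores the state and calls ToggleActive, which also runs from the construction script.
; ToggleActive lazily creates a dynamic material on the gate mesh, tints it blue or red, and switches the nav modifier between default and null areas.
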(event EventToggleGate
  (params (Active :type Boolean))
  (Variables|Default|SetActive Active)
  (CallFunction|ToggleActive))

(fn ConstructionScript
  (CallFunction|ToggleActive))

(fn ToggleActive
  (bind _active (Variables|Default|GetActive))
  (Utilities|IsValid (Variables|Default|GetM_Gate)
    (:Is%20Valid
      _)
    (:Is%20Not%20Valid
      (bind _returnvalue (Rendering|Material|CreateDynamicMaterialInstance (Variables|Default|GetSM_Large_Gate_01) 1 0 "None" :!class /Script/Engine.PrimitiveComponent))
      (Variables|Default|SetM_Gate _returnvalue)))
  (Rendering|Material|SetVectorParameterValue (Variables|Default|GetM_Gate) "Color_Tint_R" (Math|Color|SelectColor "(R=0.000000,G=0.066626,B=1.000000,A=1.000000)" "(R=1.000000,G=0.000000,B=0.000000,A=1.000000)" _active) :!class /Script/Engine.MaterialInstanceDynamic)
  (Class|NavModifierComponent|SetAreaClass (Variables|Default|GetNavModifier) (select _active "/Script/NavigationSystem.NavArea_Default" "/Script/NavigationSystem.NavArea_Null")))