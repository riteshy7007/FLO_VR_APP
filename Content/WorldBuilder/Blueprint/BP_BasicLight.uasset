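; BP_BasicLight is a light Blueprint whose color and brightness can be changed through events.
; The construction script sets the light component to StartingIntensity.
; UpdateLightColor applies a new color, and UpdateLightIntensity maps a 0–1 alpha onto a clamped range from zero to StartingIntensity, so that variable acts as the maximum brightness.
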(event EventBeginPlay)

(event Collision|EventActorBeginOverlap
  (params (OtherActor :type Actor%20Object%20Reference)))

(event EventTick
  (params (DeltaSeconds :type Float%20%28single-precision%29)))

(event EventUpdateLightColor
  (params (NewColor :type Linear%20Color%20Structure))
  (Rendering|Components|Light|SetLightColor (Variables|Default|GetLightComponent0) NewColor true))

(event EventUpdateLightIntensity
  (params (Alpha :type Float%20%28single-precision%29))
  (Rendering|Components|Light|SetIntensity (Variables|Default|GetLightComponent0) (Math|Float|MapRangeClamped Alpha 0.0 1.0 0.0 (Variables|Default|GetStartingIntensity))))

(fn ConstructionScript
  (Rendering|Components|Light|SetIntensity (Variables|Default|GetLightComponent0) (Variables|Default|GetStartingIntensity)))