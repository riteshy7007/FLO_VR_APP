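; BP_IslandGaze is a gate Blueprint whose forcefield is toggled through a button, apparently by the player's gaze.
; ToggleGate receives a component and, if it is SMButtonAPush, immediately flips GateIsOpen, switching forcefield visibility and the collision of gate, frame and forcefield.
; Any other component clears ButtonInFocus.
; A three-second gaze dwell check using Delay exists but is disconnected, so it never runs.
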(event Custom|ToggleGate
  (params (Component :type Primitive%20Component%20Object%20Reference))
  ;[1 1 1] Check if user is looking at the button
  (if (== Component (Variables|Default|GetSM_Button_A_Push))
    ;[1 1 1] Toggle the gate between open and closed. If the forcefield was closed but wants to open, hide forcefield and turn off collisions. If it was open, but now wants to close, show the forcefield and turn back on collisions.
    (Rendering|SetVisibility (Variables|Default|GetSM_Large_Gate_Forcefield) (Variables|Default|GetGateIsOpen) false)
    (Collision|SetCollisionEnabled (Variables|Default|GetSM_Large_Gate_Frame) (select (Variables|Default|GetGateIsOpen) "QueryAndPhysics" "NoCollision"))
    (Variables|Default|SetGateIsOpen (not (Variables|Default|GetGateIsOpen)))
    (else
      ;[1 1 1] If user looks away after looking at the buttons, set back to off.
      (if (Variables|Default|GetButtonInFocus)
        (Variables|Default|SetButtonInFocus false)))))

(event EventBeginPlay)

(event Collision|EventActorBeginOverlap
  (params (OtherActor :type Actor%20Object%20Reference)))

(event EventTick
  (params (DeltaSeconds :type Float%20%28single-precision%29)))

(fn ConstructionScript)