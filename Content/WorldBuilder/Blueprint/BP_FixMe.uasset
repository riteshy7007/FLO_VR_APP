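; BP_FixMe is an interactive puzzle cube that opens into an exploded view and can be fixed with a puzzle piece.
; A timeline Alpha drives Explode, pushing cached Arrow components outward and swinging the front wall, previewable via ShowExploded in construction.
; Overlapping a non-cube BP_PuzzlePiece destroys it, starts sphere rotation, then after delays shows the shield, lights the emissive and closes.
; Status requests play a sound reflecting Fixed.
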(event OnComponentBeginOverlap(Sphere)
  (params (OverlappedComponent :type Primitive%20Component%20Object%20Reference) (OtherActor :type Actor%20Object%20Reference) (OtherComp :type Primitive%20Component%20Object%20Reference) (OtherBodyIndex :type Integer) (bFromSweep :type Boolean) (SweepResult :type Hit%20Result%20Structure%20%28by%20ref%29))
  ;[1 1 1] We need to be sure that this is only activated when the correct Blueprint overlaps with the sphere
  ;[1 1 1] If the cube overlaps, will return true and do nothing. If the sphere overlaps, the first cast will fail and the second will succed
  (Utilities|Casting|CastToBP_PuzzlePiece_Cube OtherActor
    (:CastFailed
      (bind _asbp_puzzle_piece (Utilities|Casting|CastToBP_PuzzlePiece OtherActor))
      ;[1 1 1] Once fixed is true, the collision is no longer needed
      (if (not (Variables|Default|GetFixed))
        ;[1 1 1] Delete the approved, overlapped actor
        (Actor|DestroyActor _asbp_puzzle_piece)
        ;[1 1 1] When true, EventTick will rotate the sphere
        (Variables|Default|SetFixed true)
        ;[1 1 1] As if charging up, wait 3 seconds and then set the "shield" to visible
        (Utilities|FlowControl|Delay 3.0)
        (Rendering|SetVisibility (Variables|Default|GetCylinder) true false)
        ;[1 1 1] As if charging up, wait 5 seconds and then show the sphere as charged
        (Utilities|FlowControl|Delay 5.0)
        (Rendering|Material|SetMaterial (Variables|Default|GetSM_PuzzleSphere_A) 2 "/Game/WorldBuilder/Assets/Props/PuzzlePieces/PuzzleCube_A/Material/M_PuzzleCube_A_EmissiveOn.M_PuzzleCube_A_EmissiveOn")
        ;[1 1 1] Give us time to view the "fully charged" Blueprint and then close
        (Utilities|FlowControl|Delay 1e+01)
        (CallFunction|CloseCube)))))

(event Custom|Close%20Cube
  ;[1 1 1] Using a single float value, we can interpolate between closed and exploded
  (bind (_direction _alpha) (Timeline|Timeline_OpenClose ReverseFromEnd)
    (:Update
      (Variables|Default|SetAlpha _alpha)
      (CallFunction|Explode))
    (:Finished
      (Variables|Default|SetisExploded (Utilities|Enum|Equal(Enum) _direction "Forward")))))

(event Custom|OpenCube
  ;[1 1 1] Using a single float value, we can interpolate between closed and exploded
  (bind (_direction _alpha) (Timeline|Timeline_OpenClose PlayFromStart)
    (:Update
      (Variables|Default|SetAlpha _alpha)
      (CallFunction|Explode))
    (:Finished
      (Variables|Default|SetisExploded (Utilities|Enum|Equal(Enum) _direction "Forward")))))

(event EventBeginPlay
  ;[1 1 1] If ShowExploded is true, set it to false and reset BP
  (if (Variables|Default|GetShowExploded)
    (Variables|Default|SetShowExploded false)
    (Variables|Default|SetAlpha 0.0)
    (CallFunction|Explode)
    (CallFunction|GetStartingData)))

(event EventTick
  (params (DeltaSeconds :type Float%20%28single-precision%29))
  ;[1 1 1] When fixed, slowly rotate the sphere
  (if (Variables|Default|GetFixed)
    (Transformation|AddLocalRotation (Variables|Default|GetSM_PuzzleSphere_A) "1.000000,1.500000,-1.000000" false false)))

(event EventInteractwithObject
  (params (RightHand :type Boolean))
  ;[1 1 1] Called from user interaction. Will not start/end the animation if animation is currently playing
  (if (not (Audio|Components|Audio|IsPlaying (Variables|Default|GetTimeline_OpenClose)))
    (if (Variables|Default|GetisExploded)
      (CallFunction|CloseCube)
      (else
        (CallFunction|OpenCube)))))

(event EventGiveStatusUpdate
  (bind _audio (Variables|Default|GetAudio))
  ;[1 1 1] When requested by the user, play a sptialized sound to indicate status
  (Audio|Components|Audio|SetSound _audio (select (Variables|Default|GetFixed) "/Game/WorldBuilder/Assets/Sounds/BeepBeepBeep.BeepBeepBeep" "/Game/WorldBuilder/Assets/Sounds/Attention.Attention"))
  (Audio|Components|Audio|Play _audio 0.0))

(fn ConstructionScript
  (CallFunction|GetStartingData)
  (Variables|Default|SetAlpha (Math|Float|SelectFloat 1.0 0.0 (Variables|Default|GetShowExploded)))
  (CallFunction|Explode)
  (if (Variables|Default|GetFixed)
    (Rendering|SetVisibility (Variables|Default|GetCylinder) true false)
    (Rendering|Material|SetMaterial (Variables|Default|GetSM_PuzzleSphere_A) 2 "/Game/WorldBuilder/Assets/Props/PuzzlePieces/PuzzleCube_A/Material/M_PuzzleCube_A_EmissiveOn.M_PuzzleCube_A_EmissiveOn")))

(fn Explode
  ;[1 1 1] The Keys being all the arrowComponents, ForEachLoop to move each
  (bind _keys (Utilities|Map|Keys (Variables|Default|GetStartingLocation)))
  (for (_array_element _array_index) _keys
    ;[1 1 1] Get the starting location of the arrowComponens and move them 25cm in their forward direction based on 0 to 1 alpha
    (bind _values (Utilities|Map|Values (Variables|Default|GetStartingLocation)))
    (Transformation|SetWorldLocation _array_element (Math|Vector|Lerp(Vector) (Utilities|Array|Get(acopy) _values _array_index) (+ (Utilities|Array|Get(acopy) _values _array_index) (* (Math|Vector|GetForwardVector _array_element) 25.0)) (Variables|Default|GetAlpha)) false false))
  ;[1 1 1] Open the 'front' wall by rotating it around the platform
  (Transformation|SetRelativeRotation (Variables|Default|GetArrow25) (Math|Rotator|Lerp(Rotator) "0,-90.000000, 0" "0.000000,90.000000,90.000000" (Variables|Default|GetAlpha) true) false false))

(fn GetStartingData
  ;[1 1 1] Clear the array before caching new data
  (Utilities|Map|Clear (Variables|Default|GetStartingLocation))
  ;[1 1 1] Get all the arrowComponents in the Blueprint and cache a reference to them and their world location
  (for _array_element (Actor|GetComponentsByClass "/Script/Engine.ArrowComponent")
    (Utilities|Map|Add (Variables|Default|GetStartingLocation) _array_element (Transformation|GetWorldLocation _array_element))))