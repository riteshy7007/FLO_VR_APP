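; BP_Speaker is a speaker actor that repeatedly plays an assignable sound at random intervals.
; The construction script assigns the Sound variable to the Audio component.
; If IsActive is set on BeginPlay, a self-calling PlayAudio event waits a random delay, plays the audio and repeats indefinitely.
; Poking its UX Tools pressable button only plays a 2D press sound, without affecting the loop.
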(event OnBeginPoke(UxtPressableButton)
  (params (Button :type Uxt%20Pressable%20Button%20Component%20Object%20Reference) (Pointer :type Uxt%20Near%20Pointer%20Component%20Object%20Reference))
  (Audio|PlaySound2D "/Game/WorldBuilder/Assets/Sounds/Press.Press" 1.0 1.0 0.0 0 0))

(event Custom|PlayAudio
  ;[1 1 1] When called, it will play the audio after a random delay forever.
  (Utilities|FlowControl|Delay (Math|Random|RandomFloatinRange 5.0 15.0))
  (Audio|Components|Audio|Play (Variables|Default|GetAudio) 0.0)
  (CallFunction|PlayAudio))

(event EventBeginPlay
  ;[1 1 1] IfActive, play the audio
  (if (Variables|Default|GetisActive)
    (CallFunction|PlayAudio)))

(event Collision|EventActorBeginOverlap
  (params (OtherActor :type Actor%20Object%20Reference)))

(event EventTick
  (params (DeltaSeconds :type Float%20%28single-precision%29)))

(fn ConstructionScript
  (Audio|Components|Audio|SetSound (Variables|Default|GetAudio) (Variables|Default|GetSound)))