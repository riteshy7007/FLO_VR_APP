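; HoloLens panel actor that steps through a sequence of UMG instruction panels with checkpoints, a title pin and a Next button.
; BuildPanel creates each widget from PanelData, initializes its checkpoint state and enables Next immediately when there are no points.
; A game mode event supplies "Actor,Socket" strings, resolved to tool mesh sockets that a spawned spline tracks from the panel every Tick.
; Helper functions yaw the panel toward the HMD camera.
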(event Custom|SplineTargetChanged
  (params (Target%20details :type String))
  (CallFunction|SetSplineTarget Target%20details))

(event EventBeginPlay
  (bind _asbp_panel_title (Utilities|Casting|CastToBP_PanelTitle (UserInterface|GetUserWidgetObject (Variables|Default|GetPanel%20Title))))
  (Variables|/Game/FLO/Blueprint/PanelBluprint/BP_PanelTitle.BP_PanelTitle_C|SetParent%20PanelBP _asbp_panel_title self)
  (bind _returnvalue (Game|SpawnActorfromClass "/Game/FLO/Blueprint/Features/BPSpline.BPSpline_C" (Math|Transform|MakeTransform "0, 0, 0") "Undefined" 0 0))
  (bind _output_get (Variables|Default|SetPanelSPline _returnvalue))
  (bind _output_get_2 (Variables|/Game/FLO/Blueprint/Features/BPSpline.BPSpline_C|SetStartTransform _output_get (Variables|Default|GetemptyTransform)))
  (Variables|/Game/FLO/Blueprint/Features/BPSpline.BPSpline_C|SetEndTransform _output_get _output_get_2)
  (bind _asgm_holo_lens (Utilities|Casting|CastToGM_HoloLens (Game|GetGameMode)))
  (EventDispatchers|BindEventtoSplineTargetChanged _asgm_holo_lens (delegate Custom|SplineTargetChanged)))

(event Collision|EventActorBeginOverlap
  (params (OtherActor :type Actor%20Object%20Reference)))

(event EventTick
  (params (DeltaSeconds :type Float%20%28single-precision%29))
  (CallFunction|UpdatePanelSpline))

(fn ConstructionScript)

(fn BuildPanel
  (params (PanelInfo :type Panel%20Info%20Struct%20Structure))
  (bind (_umgpanelwidgetclass _panelname) (Utilities|Struct|BreakPanelInfoStruct PanelInfo))
  (bind _panel_data (Variables|Default|GetPanel%20Data))
  (bind _panelissequencelist (Variables|/Script/WorldBuilder.PanelInfoData|GetPanelIsSequenceList _panel_data))
  (bind _currentpanelindex (Variables|/Script/WorldBuilder.PanelInfoData|GetcurrentPanelIndex _panel_data))
  (bind _returnvalue (Utilities|Array|Length _panelissequencelist))
  (bind _returnvalue_2 (UserInterface|CreateWidget _umgpanelwidgetclass))
  (bind _asbp_base_umgwidget (Utilities|Casting|CastToBP_BaseUMGWidget _returnvalue_2))
  (Variables|/Game/FLO/Blueprint/PanelBluprint/BP_PanelDefault.BP_PanelDefault_C|SetPanel%20Index (Default|GetPanelDefaults _asbp_base_umgwidget) _currentpanelindex)
  (Variables|/Game/FLO/Blueprint/PanelBluprint/BP_PanelDefault.BP_PanelDefault_C|SetPanelCount (Default|GetPanelDefaults _asbp_base_umgwidget) _returnvalue)
  (Default|ConstructPanelDefault (Default|GetPanelDefaults _asbp_base_umgwidget) _currentpanelindex _returnvalue)
  (CallFunction|IntializePanelPointList _panelname _asbp_base_umgwidget)
  (UserInterface|SetWidget (Variables|Default|GetPanelInfo) _asbp_base_umgwidget)
  (CallFunction|IntializeNextButton _asbp_base_umgwidget))

(fn IntializeNextButton
  (params (UMG%20panel%20Widget :type BP%20Base%20UMG%20Widget%20Object%20Reference))
  (bind _asbpnext_button (Utilities|Casting|CastToBPNextButton (UserInterface|GetUserWidgetObject (Variables|Default|GetNextButton))))
  (Variables|/Game/FLO/Blueprint/PanelBluprint/BPNextButton.BPNextButton_C|SetCurrentPanelBP _asbpnext_button self)
  (bind _filterpointlist (Default|FetchAllPoints UMG%20panel%20Widget))
  (if (== (Utilities|Array|Length _filterpointlist) 0)
    (Variables|Default|SetAllPointsChecked true)
    (CallFunction|CallNextButtonStateChange)))

(fn CallNextButtonStateChange
  (bind _asbpnext_button (Utilities|Casting|CastToBPNextButton (UserInterface|GetUserWidgetObject (Variables|Default|GetNextButton))))
  (Default|ToggleNextButtonActivation _asbpnext_button (Variables|Default|GetAllPointsChecked)))

(fn IntializePanelPointList
  (params (PanelName :type String) (PanelUserWidgetObject :type BP%20Base%20UMG%20Widget%20Object%20Reference))
  (bind _panel_data (Variables|Default|GetPanel%20Data))
  (bind _panel_data_2 (Variables|Default|GetPanel%20Data))
  (bind _pointlistinfoarray (LocalVariables|GetPointListInfoArray))
  (bind _returnvalue (Class|PanelInfoData|GetPanelInfobyName _panel_data))
  (bind _returnvalue_2 (Class|PanelInfoData|GetPanelInfobyName _panel_data_2 PanelName))
  (bind _panelpointlist (Utilities|Struct|BreakPanelInfoStruct _returnvalue))
  (bind (_umgpanelwidgetclass _panelname) (Utilities|Struct|BreakPanelInfoStruct _returnvalue_2))
  (bind _returnvalue_3 (Utilities|Array|Length _panelpointlist))
  (bind _filterpointlist (Default|FetchAllPoints PanelUserWidgetObject))
  (if (not (== (Utilities|Array|Length _filterpointlist) 0))
    (if (or (not (== (Utilities|Array|Length _filterpointlist) _returnvalue_3)) (== _returnvalue_3 0))
      (for _array_element _filterpointlist
        (Variables|/Game/FLO/Blueprint/UI/BP_PointList.BP_PointList_C|SetParentPanelBP _array_element self)
        (Utilities|Array|Clear (LocalVariables|GetPointInfoArray))
        (for _array_element_2 (Variables|/Game/FLO/Blueprint/UI/BP_PointList.BP_PointList_C|GetCheckPoints _array_element)
          (Utilities|Array|Add (LocalVariables|GetPointInfoArray) (Utilities|Struct|MakePointInfo (Class|FLOFunctionLibrary|GetRandomString) "Unchecked" false)))
        (Utilities|Array|Add (LocalVariables|GetPointListInfoArray) (Utilities|Struct|MakePointListInfo (LocalVariables|GetPointInfoArray))))
      (Class|PanelInfoData|ReplaceInfoatIndex _panel_data_2 (Utilities|Struct|MakePanelInfoStruct _umgpanelwidgetclass _panelname _pointlistinfoarray) (Class|PanelInfoData|GetPanelIndexbyName _panel_data_2 PanelName))
      (for (_array_element_3 _array_index) _filterpointlist
        (Variables|/Game/FLO/Blueprint/UI/BP_PointList.BP_PointList_C|SetListinfo _array_element_3 (Utilities|Array|Get(acopy) _pointlistinfoarray _array_index))))))

(fn Recenter
  (bind _hmdcameraref (Variables|Default|GetHMDCameraRef))
  (Utilities|IsValid _hmdcameraref
    (:Is%20Valid
      (Transformation|SetActorRotation (Math|Rotator|MakeRotator 0.0 0.0 (.yaw (Math|Rotator|FindLookatRotation (Transformation|GetWorldLocation (Variables|Default|GetScene)) (Transformation|GetWorldLocation _hmdcameraref))))))))

(fn TogglePin
  (params (ON :type Boolean))
  (Variables|Default|SetIsPinned ON)
  (bind _asbp_panel_title (Utilities|Casting|CastToBP_PanelTitle (UserInterface|GetUserWidgetObject (Variables|Default|GetPanel%20Title))))
  (Default|TogglePinTexture _asbp_panel_title ON)
  (if ON
    (Components|Activation|Deactivate (Variables|Default|GetUxtFollow))
    (else
      (Components|Activation|Deactivate (Variables|Default|GetUxtFollow)))))

(fn SetSplineTarget
  (params (TargetSpline :type String))
  (bind (_lefts _rights) (Utilities|String|Split TargetSpline ","))
  (Variables|Default|SetCurrenSplineTargetActor 0)
  (if (Utilities|Array|IsEmpty TargetSpline)
    (Variables|Default|SetCurrentSplineRelativeTargetActorTransform (Transformation|GetSocketTransform (Variables|Default|GetPanelBG) "Socket" "RTS_World"))
    (else
      (bind _asgm_holo_lens (Utilities|Casting|CastToGM_HoloLens (Game|GetGameMode)))
      (for _array_element (Variables|/Game/FLO/Core/GM_HoloLens.GM_HoloLens_C|GetToolActor _asgm_holo_lens)
        (if (Utilities|Enum|Equal(Enum) (Utilities|GetObjectName _array_element) (Utilities|String|MakeLiteralString _lefts))
          (Utilities|IsValid (Class|StaticMesh|FindSocket (Variables|/Script/Engine.StaticMeshComponent|GetStaticMesh (Variables|/Script/Engine.StaticMeshActor|GetStaticMeshComponent _array_element)) (Utilities|String|StringToName _rights))
            (:Is%20Valid
              (Variables|Default|SetCurrenSplineTargetActor _array_element)
              (Variables|Default|SetCurrentSplineRelativeTargetActorTransform (Math|Transform|MakeTransform (Variables|/Script/Engine.StaticMeshSocket|GetRelativeLocation (Class|StaticMesh|FindSocket (Variables|/Script/Engine.StaticMeshComponent|GetStaticMesh (Variables|/Script/Engine.StaticMeshActor|GetStaticMeshComponent _array_element)) (Utilities|String|StringToName _rights))) (Variables|/Script/Engine.StaticMeshSocket|GetRelativeRotation (Class|StaticMesh|FindSocket (Variables|/Script/Engine.StaticMeshComponent|GetStaticMesh (Variables|/Script/Engine.StaticMeshActor|GetStaticMeshComponent _array_element)) (Utilities|String|StringToName _rights))) (Variables|/Script/Engine.StaticMeshSocket|GetRelativeScale (Class|StaticMesh|FindSocket (Variables|/Script/Engine.StaticMeshComponent|GetStaticMesh (Variables|/Script/Engine.StaticMeshActor|GetStaticMeshComponent _array_element)) (Utilities|String|StringToName _rights))))))))))))

(fn ClearSplinePointing
  (bind _panelspline (Variables|Default|GetPanelSPline))
  (Variables|/Game/FLO/Blueprint/Features/BPSpline.BPSpline_C|SetEndTransform _panelspline (Transformation|GetSocketTransform (Variables|Default|GetPanelBG) "Socket" "RTS_World"))
  (Variables|/Game/FLO/Blueprint/Features/BPSpline.BPSpline_C|SetStartTransform _panelspline ""))

(fn UpdatePanelSpline
  (bind _panelspline (Variables|Default|GetPanelSPline))
  (bind _currensplinetargetactor (Variables|Default|GetCurrenSplineTargetActor))
  (bind _currentsplinerelativetargetactortransform (Variables|Default|GetCurrentSplineRelativeTargetActorTransform))
  (bind _panelspline_2 (Variables|Default|GetPanelSPline))
  (bind _returnvalue (Transformation|GetActorTransform _currensplinetargetactor))
  (bind (_location _rotation) (Math|Transform|BreakTransform _currentsplinerelativetargetactortransform))
  (Utilities|IsValid (Variables|Default|GetCurrenSplineTargetActor)
    (:Is%20Valid
      (Variables|/Game/FLO/Blueprint/Features/BPSpline.BPSpline_C|SetStartTransform _panelspline_2 (Transformation|GetSocketTransform (Variables|Default|GetPanelBG) "None" "RTS_World"))
      (Variables|/Game/FLO/Blueprint/Features/BPSpline.BPSpline_C|SetEndTransform _panelspline_2 (Math|Transform|MakeTransform (Math|Transform|TransformLocation _returnvalue _location) (Math|Transform|TransformRotation _returnvalue _rotation))))
    (:Is%20Not%20Valid
      (Variables|/Game/FLO/Blueprint/Features/BPSpline.BPSpline_C|SetStartTransform _panelspline "")
      (Variables|/Game/FLO/Blueprint/Features/BPSpline.BPSpline_C|SetEndTransform _panelspline ""))))

(fn LookatPlayer
  (Utilities|IsValid (Variables|Default|GetHMDCameraRef)
    (:Is%20Valid
      (Transformation|SetActorRotation (Math|Rotator|MakeRotator 0.0 0.0 (.Yaw (Math|Rotator|BreakRotator (Math|Rotator|FindLookatRotation (Transformation|GetWorldLocation (Variables|Default|GetScene)) (Transformation|GetWorldLocation (Variables|Default|GetHMDCameraRef))))))))))

(fn BuildNextPanel
  (bind _panel_data (Variables|Default|GetPanel%20Data))
  (if (< (Variables|/Script/WorldBuilder.PanelInfoData|GetcurrentPanelIndex _panel_data) (Utilities|Array|Length (Variables|/Script/WorldBuilder.PanelInfoData|GetPanelIsSequenceList _panel_data)))
    (CallFunction|BuildPanel (Class|PanelInfoData|MovetoNextPanelData _panel_data))))

(fn BuildPanelAT
  (params (Index :type Integer))
  (CallFunction|BuildPanel (Class|PanelInfoData|MovetoPanelData (Variables|Default|GetPanel%20Data) Index)))