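; Mixed-reality status panel actor that hosts a BP_StatusPanelDefaults widget.
; On BeginPlay it hands the widget a reference to itself and has it build the panel list.
; Opening shows the panel pinned with collision on, then recenters it at an offset in front of the HMD camera, yawed toward the player.
; Pinning updates the widget's pin texture and deactivates UxtFollow; unpinning reactivates following.
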(event EventBeginPlay
  (CallFunction|BuildPanelItems)
  (bind _asbp_status_panel_defaults (Utilities|Casting|CastToBP_StatusPanelDefaults (UserInterface|GetUserWidgetObject (Variables|Default|GetPanelInfo))))
  (Variables|Default|SetAs%20BP%20Status%20Panel%20Defaults _asbp_status_panel_defaults))

(event Collision|EventActorBeginOverlap
  (params (OtherActor :type Actor%20Object%20Reference)))

(event EventTick
  (params (DeltaSeconds :type Float%20%28single-precision%29)))

(fn ConstructionScript)

(fn Recenter
  (bind _hmdcameraref (Variables|Default|GetHMDCameraRef))
  (bind _scene (Variables|Default|GetScene))
  (Utilities|IsValid _hmdcameraref
    (:Is%20Valid
      (Transformation|SetWorldLocation _scene (+ (* (Math|Vector|GetForwardVector _hmdcameraref) 8e+01) (Transformation|GetWorldLocation _hmdcameraref)) false false)
      (Transformation|AddLocalOffset _scene "0,30.000000,-15.000000" false false)
      (CallFunction|LookatthePlayer))))

(fn BuildPanelItems
  (bind _asbp_status_panel_defaults (Utilities|Casting|CastToBP_StatusPanelDefaults (UserInterface|GetUserWidgetObject (Variables|Default|GetPanelInfo))))
  (Variables|/Game/FLO/Blueprint/PanelBluprint/BP_StatusPanelDefaults.BP_StatusPanelDefaults_C|SetParent%20Status%20panel%20Reference _asbp_status_panel_defaults self)
  (Default|ConstructPanelList _asbp_status_panel_defaults))

(fn LookatthePlayer
  (bind _hmdcameraref (Variables|Default|GetHMDCameraRef))
  (Utilities|IsValid _hmdcameraref
    (:Is%20Valid
      (Transformation|SetActorRotation (Math|Rotator|MakeRotator 0.0 0.0 (.yaw (Math|Rotator|FindLookatRotation (Transformation|GetWorldLocation (Variables|Default|GetScene)) (Transformation|GetWorldLocation _hmdcameraref))))))))

(fn TogglePin
  (params (Pinned :type Boolean))
  (bind _uxtfollow (Variables|Default|GetUxtFollow))
  (Variables|Default|SetIs%20Pinned Pinned)
  (bind _asbp_status_panel_defaults (Utilities|Casting|CastToBP_StatusPanelDefaults (UserInterface|GetUserWidgetObject (Variables|Default|GetPanelInfo))))
  (Default|TogglePinTexture _asbp_status_panel_defaults Pinned)
  (if Pinned
    (Components|Activation|Deactivate _uxtfollow)
    (else
      (Components|Activation|Activate _uxtfollow true))))

(fn OpenStatuspanel
  (Rendering|SetActorHiddenInGame false)
  (CallFunction|TogglePin true)
  (Collision|SetActorEnableCollision true)
  (CallFunction|Recenter))