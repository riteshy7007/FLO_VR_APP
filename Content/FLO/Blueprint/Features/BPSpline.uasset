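; BPSpline is an actor that shapes a single spline mesh between a start and an end transform.
; The construction script creates a dynamic instance of BasicShapeMaterial, then calls ConstructSpline to set the mesh endpoints.
; Each tangent is that transform's forward vector multiplied by its scale and the distance between endpoints.
; ConstructSpline also sets the material's Strip Tiling to a fixed zero; the event graph is inactive.
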(event EventBeginPlay)

(event Collision|EventActorBeginOverlap
  (params (OtherActor :type Actor%20Object%20Reference)))

(event EventTick
  (params (DeltaSeconds :type Float%20%28single-precision%29)))

(fn ConstructionScript
  (bind _returnvalue (Rendering|Material|CreateDynamicMaterialInstance (Variables|Default|GetSplineMesh) 0 "/Game/FLO/Meshes/BasicShapeMaterial.BasicShapeMaterial" "None" :!class /Script/Engine.PrimitiveComponent))
  (Variables|Default|SetSpline%20Material%20Dynamic _returnvalue)
  (CallFunction|ConstructSpline))

(fn ConstructSpline
  (bind _endtransform (Variables|Default|GetEndTransform))
  (bind _starttransform (Variables|Default|GetStartTransform))
  (bind (_location _rotation _scale) (Math|Transform|BreakTransform _starttransform))
  (bind (_location_2 _rotation_2 _scale_2) (Math|Transform|BreakTransform _endtransform))
  (bind _returnvalue (- _location _location_2))
  (bind _returnvalue_2 (Math|Vector|VectorLength _returnvalue))
  (SplineMesh|SetStartandEnd (Variables|Default|GetSplineMesh) _location (* (* (Math|Vector|GetForwardVector _rotation) _scale) _returnvalue_2) _location_2 (* (* (Math|Vector|GetForwardVector _rotation_2) _scale_2) _returnvalue_2) true :!class /Script/Engine.SplineMeshComponent)
  (Rendering|Material|SetScalarParameterValue (Variables|Default|GetSpline%20Material%20Dynamic) "Strip Tiling" 0.0 :!class /Script/Engine.MaterialInstanceDynamic))