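; Status panel actor that shows a list widget in the world and can turn to face the player's headset camera.
; BuildPanelItems casts the PanelInfo widget to BP_StatusPanelDefaults, hands it a reference to this panel and has it construct its list.
; LookAtThePlayer rotates the actor on yaw only toward HMDCameraRef, keeping it upright.
; Recenter and TogglePin are empty, and the event graph has no active logic.
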(event EventBeginPlay)

(event Collision|EventActorBeginOverlap
  (params (OtherActor :type Actor%20Object%20Reference)))

(event EventTick
  (params (DeltaSeconds :type Float%20%28single-precision%29)))

(fn ConstructionScript)

(fn Recenter)

(fn BuildPanelItems
  (bind _asbp_status_panel_defaults (Utilities|Casting|CastToBP_StatusPanelDefaults (UserInterface|GetUserWidgetObject (Variables|Default|GetPanelInfo))))
  (Variables|/Game/FLO/Blueprint/PanelBluePrints/BP_StatusPanelDefaults.BP_StatusPanelDefaults_C|SetParent%20Status%20panel%20Reference _asbp_status_panel_defaults self)
  (Default|ConstructPanelList _asbp_status_panel_defaults))

(fn LookatthePlayer
  (bind _hmdcameraref (Variables|Default|GetHMDCameraRef))
  (Utilities|IsValid _hmdcameraref
    (:Is%20Valid
      (Transformation|SetActorRotation (Math|Rotator|MakeRotator 0.0 0.0 (.yaw (Math|Rotator|FindLookatRotation (Transformation|GetWorldLocation (Variables|Default|GetScene)) (Transformation|GetWorldLocation _hmdcameraref))))))))

(fn TogglePin)