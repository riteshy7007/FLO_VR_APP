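; HoloLens panel actor that shows a sequence of UMG panel widgets from PanelData, with next-panel and jump-to-index builds.
; BuildPanel creates each widget, sets its index and count, and links the Next button, marking points checked when none exist.
; A spline can point from the panel to a named socket on a tool actor.
; It yaws toward the headset; pinning updates the title, though both states deactivate UxtFollow.
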(event EventBeginPlay)

(event Collision|EventActorBeginOverlap
  (params (OtherActor :type Actor%20Object%20Reference)))

(event EventTick
  (params (DeltaSeconds :type Float%20%28single-precision%29)))

(fn ConstructionScript)

(fn BuildPanel
  (params (PanelInfo :type Panel%20Info%20Struct%20Structure))
  (bind (_umgpanelwidgetclass _panelname) (Utilities|Struct|BreakPanelInfoStruct PanelInfo))
  (bind _panel_data (Variables|Default|GetPanel%20Data))
  (bind _panelissequencelist (Variables|/Script/WorldBuilder.PanelInfoData|GetPanelIsSequenceList _panel_data))
  (bind _currentpanelindex (Variables|/Script/WorldBuilder.PanelInfoData|GetcurrentPanelIndex _panel_data))
  (bind _returnvalue (Utilities|Array|Length _panelissequencelist))
  (bind _returnvalue_2 (UserInterface|CreateWidget _umgpanelwidgetclass))
  (bind _asbp_base_umgwidget (Utilities|Casting|CastToBP_BaseUMGWidget _returnvalue_2))
  (Variables|/Game/FLO/Blueprint/PanelBluePrints/BP_PanelDefault.BP_PanelDefault_C|SetPanel%20Index (Default|GetPanelDefaults _asbp_base_umgwidget) _currentpanelindex)
  (Variables|/Game/FLO/Blueprint/PanelBluePrints/BP_PanelDefault.BP_PanelDefault_C|SetPanelCount (Default|GetPanelDefaults _asbp_base_umgwidget) _returnvalue)
  (Default|ConstructPanelDefault (Default|GetPanelDefaults _asbp_base_umgwidget) _currentpanelindex _returnvalue)
  (CallFunction|IntializePanelPointList _panelname _asbp_base_umgwidget)
  (UserInterface|SetWidget (Variables|Default|GetPanelInfo) _asbp_base_umgwidget)
  (CallFunction|IntializeNextButton _asbp_base_umgwidget))

(fn IntializeNextButton
  (params (UMG%20panel%20Widget :type BP%20Base%20UMG%20Widget%20Object%20Reference))
  (bind _asbp_panel_nextbutton (Utilities|Casting|CastToBP_PanelNextbutton (UserInterface|GetUserWidgetObject (Variables|Default|GetNextButton))))
  (Variables|/Game/FLO/Blueprint/UI/BP_PanelNextbutton.BP_PanelNextbutton_C|SetCurrentpanel%20BP _asbp_panel_nextbutton self)
  (bind _filterpointlist (Default|FetchAllPoints UMG%20panel%20Widget))
  (if (== (Utilities|Array|Length _filterpointlist) 0)
    (Variables|Default|SetAllPointsChecked true)))

(fn CallNextButtonStateChange
  (bind _asbp_panel_nextbutton (Utilities|Casting|CastToBP_PanelNextbutton (UserInterface|GetUserWidgetObject (Variables|Default|GetNextButton))))
  (Default|ToggleNextButton _asbp_panel_nextbutton (Variables|Default|GetAllPointsChecked)))

(fn IntializePanelPointList
  (params (PanelName :type String) (PanelUserWidgetObject :type BP%20Base%20UMG%20Widget%20Object%20Reference)))

(fn Recenter
  (bind _hmdcameraref (Variables|Default|GetHMDCameraRef))
  (Utilities|IsValid _hmdcameraref
    (:Is%20Valid
      (Transformation|SetActorRotation (Math|Rotator|MakeRotator 0.0 0.0 (.yaw (Math|Rotator|FindLookatRotation (Transformation|GetWorldLocation (Variables|Default|GetScene)) (Transformation|GetWorldLocation _hmdcameraref))))))))

(fn TogglePin
  (params (ON :type Boolean))
  (Variables|Default|SetIsPinned ON)
  (bind _asbp_panel_title (Utilities|Casting|CastToBP_PanelTitle (UserInterface|GetUserWidgetObject (Variables|Default|GetPanel%20Title))))
  (Default|TogglePinTexture _asbp_panel_title ON)
  (if ON
    (Components|Activation|Deactivate (Variables|Default|GetUxtFollow))
    (else
      (Components|Activation|Deactivate (Variables|Default|GetUxtFollow)))))

(fn SetSplineTarget
  (params (TargetSpline :type String))
  (bind (_lefts _rights) (Utilities|String|Split TargetSpline ","))
  (Variables|Default|SetCurrenSplineTargetActor 0)
  (if (Utilities|Array|IsEmpty TargetSpline)
    (Variables|Default|SetCurrentSplineRelativeTargetActorTransform (Transformation|GetSocketTransform (Variables|Default|GetPanelBG) "Socket" "RTS_World"))
    (else
      (bind _asgm_holo_lens (Utilities|Casting|CastToGM_HoloLens (Game|GetGameMode)))
      (for _array_element (Variables|/Game/FLO/Core/GM_HoloLens.GM_HoloLens_C|GetToolActor _asgm_holo_lens)
        (if (Utilities|Enum|Equal(Enum) (Utilities|GetObjectName _array_element) (Utilities|String|MakeLiteralString _lefts))
          (Utilities|IsValid (Class|StaticMesh|FindSocket (Variables|/Script/Engine.StaticMeshComponent|GetStaticMesh (Variables|/Script/Engine.StaticMeshActor|GetStaticMeshComponent _array_element)) (Utilities|String|StringToName _rights))
            (:Is%20Valid
              (Variables|Default|SetCurrenSplineTargetActor _array_element)
              (Variables|Default|SetCurrentSplineRelativeTargetActorTransform (Math|Transform|MakeTransform (Variables|/Script/Engine.StaticMeshSocket|GetRelativeLocation (Class|StaticMesh|FindSocket (Variables|/Script/Engine.StaticMeshComponent|GetStaticMesh (Variables|/Script/Engine.StaticMeshActor|GetStaticMeshComponent _array_element)) (Utilities|String|StringToName _rights))) (Variables|/Script/Engine.StaticMeshSocket|GetRelativeRotation (Class|StaticMesh|FindSocket (Variables|/Script/Engine.StaticMeshComponent|GetStaticMesh (Variables|/Script/Engine.StaticMeshActor|GetStaticMeshComponent _array_element)) (Utilities|String|StringToName _rights))) (Variables|/Script/Engine.StaticMeshSocket|GetRelativeScale (Class|StaticMesh|FindSocket (Variables|/Script/Engine.StaticMeshComponent|GetStaticMesh (Variables|/Script/Engine.StaticMeshActor|GetStaticMeshComponent _array_element)) (Utilities|String|StringToName _rights))))))))))))

(fn ClearSplinePointing
  (bind _panelspline (Variables|Default|GetPanelSPline))
  (Variables|/Game/FLO/Blueprint/Features/BPSpline.BPSpline_C|SetEndTransform _panelspline (Transformation|GetSocketTransform (Variables|Default|GetPanelBG) "Socket" "RTS_World"))
  (Variables|/Game/FLO/Blueprint/Features/BPSpline.BPSpline_C|SetStartTransform _panelspline ""))

(fn UpdatePanelSpline
  (bind _panelspline (Variables|Default|GetPanelSPline))
  (bind _currensplinetargetactor (Variables|Default|GetCurrenSplineTargetActor))
  (bind _currentsplinerelativetargetactortransform (Variables|Default|GetCurrentSplineRelativeTargetActorTransform))
  (bind _panelspline_2 (Variables|Default|GetPanelSPline))
  (bind _returnvalue (Transformation|GetActorTransform _currensplinetargetactor))
  (bind (_location _rotation) (Math|Transform|BreakTransform _currentsplinerelativetargetactortransform))
  (Utilities|IsValid (Variables|Default|GetCurrenSplineTargetActor)
    (:Is%20Valid
      (Variables|/Game/FLO/Blueprint/Features/BPSpline.BPSpline_C|SetStartTransform _panelspline_2 (Transformation|GetSocketTransform (Variables|Default|GetPanelBG) "None" "RTS_World"))
      (Variables|/Game/FLO/Blueprint/Features/BPSpline.BPSpline_C|SetEndTransform _panelspline_2 (Math|Transform|MakeTransform (Math|Transform|TransformLocation _returnvalue _location) (Math|Transform|TransformRotation _returnvalue _rotation))))
    (:Is%20Not%20Valid
      (Variables|/Game/FLO/Blueprint/Features/BPSpline.BPSpline_C|SetStartTransform _panelspline "")
      (Variables|/Game/FLO/Blueprint/Features/BPSpline.BPSpline_C|SetEndTransform _panelspline ""))))

(fn LookatPlayer
  (Utilities|IsValid (Variables|Default|GetHMDCameraRef)
    (:Is%20Valid
      (Transformation|SetActorRotation (Math|Rotator|MakeRotator 0.0 0.0 (.Yaw (Math|Rotator|BreakRotator (Math|Rotator|FindLookatRotation (Transformation|GetWorldLocation (Variables|Default|GetScene)) (Transformation|GetWorldLocation (Variables|Default|GetHMDCameraRef))))))))))

(fn BuildNextPanel
  (bind _panel_data (Variables|Default|GetPanel%20Data))
  (if (< (Variables|/Script/WorldBuilder.PanelInfoData|GetcurrentPanelIndex _panel_data) (Utilities|Array|Length (Variables|/Script/WorldBuilder.PanelInfoData|GetPanelIsSequenceList _panel_data)))
    (CallFunction|BuildPanel (Class|PanelInfoData|MovetoNextPanelData _panel_data))))

(fn BuildPanelAT
  (params (Index :type Integer))
  (CallFunction|BuildPanel (Class|PanelInfoData|MovetoPanelData (Variables|Default|GetPanel%20Data) Index)))